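; Collison is a destructible actor that colors itself green or blue at BeginPlay, depending on whether its SpawnNumber matches ColorPosition.
; A Box overlap turns it red, then after a short delay calls NewPhase on RoundController, reports its SpawnNumber to the Hud and destroys itself.
; A shakeIt event offsets it through a DoOnce-guarded timeline, then restores its position.
; DestroyHit and GetsDestroyed are empty stubs.
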(event `self.ReceiveBeginPlay`
  (bind _staticmeshcomponent (`self.StaticMeshComponent`))
  ;[1 1 1] starting color
  (`KismetSystemLibrary.Delay` 0.01)
  (if (== (`self.spawnNumber`) (`self.colorPosition`))
    (`MeshComponent.SetVectorParameterValueOnMaterials` _staticmeshcomponent "Base" (0.0 1.0 0.0))
    (else
      (`MeshComponent.SetVectorParameterValueOnMaterials` _staticmeshcomponent "Base" (0.0 0.0 1.0)))))

(event `self.Box.OnComponentBeginOverlap`
  (params (OverlappedComponent :type "PrimitiveComponent Object Reference") (OtherActor :type "Actor Object Reference") (OtherComp :type "PrimitiveComponent Object Reference") (OtherBodyIndex :type Integer) (bFromSweep :type Boolean) (SweepResult :type "HitResult Structure (by ref)"))
  ;[1 1 1] GetsHit
  (`MeshComponent.SetVectorParameterValueOnMaterials` (`self.StaticMeshComponent`) "Base" (1.0 0.0 0.0))
  (`KismetSystemLibrary.Delay` 0.4)
  (bind _outactors (`GameplayStatics.GetAllActorsOfClass` "/Game/Blueprints/RoundController.RoundController_C"))
  (`/Game/Blueprints/RoundController.newPhase` _outactors)
  (bind _foundwidgets (`WidgetBlueprintLibrary.GetAllWidgetsOfClass` "/Game/Blueprints/UI/Hud.Hud_C"))
  (bind _ashud (cast `/Game/Blueprints/UI/Hud` (`KismetArrayLibrary.Array_Get` _foundwidgets)))
  (`/Game/Blueprints/UI/Hud.isDestroyed` _ashud (`self.spawnNumber`))
  (`self.K2_DestroyActor`))

(event `shakeIt`
  (bind _returnvalue (`self.K2_GetActorLocation`))
  (`/Engine/EditorBlueprintResources/StandardMacros.DoOnce` false :!label _label
    (:`Completed`
      (set `self.Position` _returnvalue)
      (bind (_direction _newtrack_1) (`Timeline|Timeline_0` :`NewTime` 0.0 :!via `PlayFromStart`)
        (:`Update`
          (`self.K2_SetActorRelativeLocation` (+ _returnvalue _newtrack_1)))
        (:`Finished`
          (`self.K2_SetActorRelativeLocation` (`self.Position`))
          (goto _label :!via `Reset`))))))

(fn `destroyHit`
  (params (destroyed :type "Float (double-precision)"))
  (returns (destroyedNumber :type "Float (double-precision)"))
  (return 0.0))

(fn `getsDestroyed`
  (params (destroyedObjectSpasnNumber :type "Float (double-precision) (by ref)"))
  (returns (number :type "Float (double-precision)"))
  (return 0.0))

(fn `UserConstructionScript`)