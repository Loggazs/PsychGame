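; Player Blueprint for a jumping game where holding a direction input charges a power bar and releasing it jumps from the origin to a rock.
; The power level picks one of three targets from that direction's RoundControllerNext array, and timeline-driven parabolic lerps, selected by GlobeStage, move the actor.
; Landing fires a shockwave, notifies the rock and may spawn a GoldenBall after checking it against the round controller.
; A separate jumpBack event reports right or wrong to the HUD and damages the landing place.
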(event `self.ReceiveBeginPlay`
  ;[1 1 1] initialize HUD
  (bind _returnvalue (`|CreateWidget` "/Game/Blueprints/UI/Hud.Hud_C"))
  (bind _output_get (set `self.HudRreference` _returnvalue))
  (`UserWidget.AddToViewport` _output_get 0)
  (`WidgetBlueprintLibrary.SetInputMode_GameOnly` (`GameplayStatics.GetPlayerController` 0)))

(event `runAnimation`
  ;[1 1 1] animation Visibility
  (`SceneComponent.SetVisibility` (`self.idle`) false false)
  (`SceneComponent.SetVisibility` (`self.run`) true false))

(event `idleanimation`
  ;[1 1 1] animation Visibility
  (`SceneComponent.SetVisibility` (`self.run`) false false)
  (`SceneComponent.SetVisibility` (`self.idle`) true false))

(event `InputAction|MoveUp`
  (params (Key :type "Key Structure" :default "AnyKey"))
  (bind _north (`self.North`))
  ;[1 1 1] North
  (:`Pressed`
    (if _north
      (`self.begin Movement` 270.0)
      (bind _aspower_bar (cast `/Game/Blueprints/UI/PowerBar` (`WidgetComponent.GetUserWidgetObject` (`self.powerbar`))))
      (bind (_direction _newtrack_0) (`Timeline|fillPowerbar` :!via `PlayFromStart` :!label _label)
        (:`Update`
          (`/Game/Blueprints/UI/PowerBar.setPower` _aspower_bar _newtrack_0)))))
  (:`Released`
    (if _north
      (`|ExecutionSequence`
        (:`then_0`
          (goto _label :!via `Stop`))
        (:`then_1`
          (`KismetSystemLibrary.Delay` 0.1)
          (bind _outactors (`GameplayStatics.GetAllActorsOfClass` "/Game/Blueprints/RoundControllerNext.RoundControllerNext_C"))
          (bind _targetposition (`self.endMovement` (`/Game/Blueprints/RoundControllerNext.North` (`KismetArrayLibrary.Array_Get` _outactors))))
          (`self.JumpOverThere` (0.0 0.0 0.0) _targetposition))))))

(event `JumpOverThere`
  (params (startPosition :type "Vector Structure") (endPosition :type "Vector Structure"))
  (switch `int` (`self.globeStage`) ; Based on Number of Globes Collected, do a different jump animation
    (:`0`
      ;[1 1 1] jump inkl landing
      (set `self.forceStrength` 0.0)
      (bind (_direction _distance _hight) (`Timeline|jumpParable1` :!via `PlayFromStart` :!label _label_2)
        (:`Update`
          (`self.K2_SetActorLocation` (+ (`KismetMathLibrary.VLerp` startPosition endPosition _distance) (`KismetMathLibrary.VLerp` (0.0 0.0 0.0) (`self.jumphight`) _hight))))
        (:`Finished`
          ;[1 1 1] after Jump Animation
          (bind _rightone (`self.checkLanding` :!label _label_3))
          (`self.shockwaveActivate`)
          (bind _asrock (cast `/Game/Blueprints/Rock` (`self.LandingPlace`)))
          (`/Game/Blueprints/Rock.Playerlanding` _asrock (`self.globeStage`))
          (`KismetSystemLibrary.Delay` 0.1)
          (if _rightone
            (`self.findGoldenGlobe`)))))
    (:`1`
      (set `self.forceStrength` 1.0)
      (bind (_direction_2 _distance_2 _hight_2) (`Timeline|jumpParable2` :!via `PlayFromStart`)
        (:`Update`
          (`self.K2_SetActorLocation` (+ (`KismetMathLibrary.VLerp` startPosition endPosition _distance_2) (`KismetMathLibrary.VLerp` (0.0 0.0 0.0) (* (`self.jumphight`) 1) _hight_2))))
        (:`Finished`
          (goto _label_3))))
    (:`2`
      (goto _label_2 :!via `PlayFromStart`))
    (:`3`
      (goto _label_2 :!via `PlayFromStart`))
    (:`4`
      (goto _label_2 :!via `PlayFromStart`))
    (:`5`
      (goto _label_2 :!via `PlayFromStart`))
    (:`6`
      (goto _label_2 :!via `PlayFromStart`))
    (:`7`
      (goto _label_2 :!via `PlayFromStart`))))

(event `InputAction|MoveRight`
  (params (Key :type "Key Structure" :default "AnyKey"))
  (bind _east (`self.East`))
  ;[1 1 1] East
  (:`Pressed`
    (if _east
      (`self.begin Movement` 180.0)
      (bind _aspower_bar (cast `/Game/Blueprints/UI/PowerBar` (`WidgetComponent.GetUserWidgetObject` (`self.powerbar`))))
      (bind (_direction _newtrack_0) (`Timeline|Timeline_0` :!via `PlayFromStart` :!label _label_4)
        (:`Update`
          (`/Game/Blueprints/UI/PowerBar.setPower` _aspower_bar _newtrack_0)))))
  (:`Released`
    (if _east
      (`|ExecutionSequence`
        (:`then_0`
          (goto _label_4 :!via `Stop`))
        (:`then_1`
          (`KismetSystemLibrary.Delay` 0.1)
          (bind _outactors (`GameplayStatics.GetAllActorsOfClass` "/Game/Blueprints/RoundControllerNext.RoundControllerNext_C"))
          (bind _targetposition (`self.endMovement` (`/Game/Blueprints/RoundControllerNext.East` (`KismetArrayLibrary.Array_Get` _outactors))))
          (`self.JumpOverThere` (0.0 0.0 0.0) _targetposition))))))

(event `jumpBack`
  (params (startPosition :type "Vector Structure") (EndPosition :type "Vector Structure"))
  (bind _hudrreference (`self.HudRreference`))
  (bind _returnvalue (`KismetSystemLibrary.GetDisplayName` (`self.LandingPlace`)))
  ;[1 1 1] jumpBack
  (bind (_direction _distance _hight) (`Timeline|Timeline_3` :!via `PlayFromStart`)
    (:`Update`
      (`self.K2_SetActorLocation` (+ (`KismetMathLibrary.VLerp` startPosition EndPosition _distance) (`KismetMathLibrary.VLerp` (0.0 0.0 0.0) (`self.jumphight`) _hight))))
    (:`Finished`
      (bind _rightone (`self.checkLanding`))
      (if _rightone
        (set `/Game/Blueprints/UI/Hud.PositionList` (`KismetStringLibrary.Concat_StrStr` _returnvalue "is Right") _hudrreference)
        (else
          (set `/Game/Blueprints/UI/Hud.PositionList` (`KismetStringLibrary.Concat_StrStr` _returnvalue " is the wrong") _hudrreference)))
      (`GameplayStatics.ApplyDamage` (`self.LandingPlace`) 500.0))))

(event `InputAction|MoveDown`
  (params (Key :type "Key Structure" :default "AnyKey"))
  (bind _south (`self.South`))
  ;[1 1 1] South
  (:`Pressed`
    (if _south
      (`self.begin Movement` 90.0)
      (bind _aspower_bar (cast `/Game/Blueprints/UI/PowerBar` (`WidgetComponent.GetUserWidgetObject` (`self.powerbar`))))
      (bind (_direction _newtrack_0) (`Timeline|Timeline_1` :!via `PlayFromStart` :!label _label_5)
        (:`Update`
          (`/Game/Blueprints/UI/PowerBar.setPower` _aspower_bar _newtrack_0)))))
  (:`Released`
    (if _south
      (`|ExecutionSequence`
        (:`then_0`
          (goto _label_5 :!via `Stop`))
        (:`then_1`
          (`KismetSystemLibrary.Delay` 0.1)
          (bind _outactors (`GameplayStatics.GetAllActorsOfClass` "/Game/Blueprints/RoundControllerNext.RoundControllerNext_C"))
          (bind _targetposition (`self.endMovement` (`/Game/Blueprints/RoundControllerNext.South` (`KismetArrayLibrary.Array_Get` _outactors))))
          (`self.JumpOverThere` (0.0 0.0 0.0) _targetposition))))))

(event `InputAction|MoveLeft`
  (params (Key :type "Key Structure" :default "AnyKey"))
  (bind _west (`self.West`))
  ;[1 1 1] West
  (:`Pressed`
    (if _west
      (`self.begin Movement` 0.0)
      (bind _aspower_bar (cast `/Game/Blueprints/UI/PowerBar` (`WidgetComponent.GetUserWidgetObject` (`self.powerbar`))))
      (bind (_direction _newtrack_0) (`Timeline|Timeline_2` :!via `PlayFromStart` :!label _label_6)
        (:`Update`
          (`/Game/Blueprints/UI/PowerBar.setPower` _aspower_bar _newtrack_0)))))
  (:`Released`
    (if _west
      (`|ExecutionSequence`
        (:`then_0`
          (goto _label_6 :!via `Stop`))
        (:`then_1`
          (`KismetSystemLibrary.Delay` 0.1)
          (bind _outactors (`GameplayStatics.GetAllActorsOfClass` "/Game/Blueprints/RoundControllerNext.RoundControllerNext_C"))
          (bind _targetposition (`self.endMovement` (`/Game/Blueprints/RoundControllerNext.West` (`KismetArrayLibrary.Array_Get` _outactors))))
          (`self.JumpOverThere` (0.0 0.0 0.0) _targetposition))))))

(fn `begin Movement`
  (params (inputdirection :type "Float (double-precision)"))
  (`SceneComponent.SetVisibility` (`self.powerbar`) true false)
  (`SceneComponent.K2_SetRelativeLocationAndRotation` (`self.powerbar`) (0.0 0.0 0.0) (`KismetMathLibrary.MakeRotator` inputdirection 90.0) false false)
  (bind _aspower_bar (cast `/Game/Blueprints/UI/PowerBar` (`WidgetComponent.GetUserWidgetObject` (`self.powerbar`))))
  (`/Game/Blueprints/UI/PowerBar.setPower` _aspower_bar 0.0))

(fn `checkLanding`
  (returns (rightOne :type Boolean))
  (bind _outactors (`GameplayStatics.GetAllActorsOfClass` "/Game/Blueprints/RoundControllerNext.RoundControllerNext_C"))
  (if (`self.North`)
    (bind _item (`KismetArrayLibrary.Array_Get` _outactors))
    (bind _north (`/Game/Blueprints/RoundControllerNext.North` _item))
    (if (not (and (`KismetArrayLibrary.Array_Contains` _north (`self.LandingPlace`)) (`KismetArrayLibrary.Array_Contains` _north (`/Game/Blueprints/RoundControllerNext.2ndElement` _item))))
      (if (`self.East`) :!label _label
        (bind _east (`/Game/Blueprints/RoundControllerNext.East` _item))
        (if (not (and (`KismetArrayLibrary.Array_Contains` _east (`self.LandingPlace`)) (`KismetArrayLibrary.Array_Contains` _east (`/Game/Blueprints/RoundControllerNext.2ndElement` _item))))
          (if (`self.South`) :!label _label_2
            (bind _south (`/Game/Blueprints/RoundControllerNext.South` _item))
            (if (not (and (`KismetArrayLibrary.Array_Contains` _south (`self.LandingPlace`)) (`KismetArrayLibrary.Array_Contains` _south (`/Game/Blueprints/RoundControllerNext.2ndElement` _item))))
              (if (`self.West`) :!label _label_3
                (bind _west (`/Game/Blueprints/RoundControllerNext.West` _item))
                (if (and (`KismetArrayLibrary.Array_Contains` _west (`self.LandingPlace`)) (`KismetArrayLibrary.Array_Contains` _west (`/Game/Blueprints/RoundControllerNext.2ndElement` _item)))
                  _
                  (else
                    (return false)))
                (else
                  (return false))))
            (else
              (goto _label_3))))
        (else
          (goto _label_2))))
    (else
      (goto _label)))
  (return true))

(fn `endMovement`
  (params (NewParam :type "Array of Actor Object Reference"))
  (returns (targetPosition :type "Vector Structure"))
  (bind _item (`KismetArrayLibrary.Array_Get` NewParam))
  (bind _item_2 (`KismetArrayLibrary.Array_Get` NewParam 1))
  (bind _item_3 (`KismetArrayLibrary.Array_Get` NewParam 2))
  (bind _returnvalue (`self.K2_GetActorLocation` _item))
  (bind _returnvalue_2 (`self.K2_GetActorLocation` _item_3))
  (bind _returnvalue_3 (< (`KismetMathLibrary.VSizeSquared` _returnvalue) (`KismetMathLibrary.VSizeSquared` _returnvalue_2)))
  (bind _aspower_bar (cast `/Game/Blueprints/UI/PowerBar` (`WidgetComponent.GetUserWidgetObject` (`self.powerbar`)))
    (:`then`
      _)
    (:`CastFailed`
      _))
  (bind _returnvalue_4 (`/Game/Blueprints/UI/PowerBar.getPower` _aspower_bar))
  (if (<= _returnvalue_4 0.33)
    (`SceneComponent.SetVisibility` (`self.powerbar`) false false)
    (if _returnvalue_3
      (set `self.LandingPlace` _item)
      (return _returnvalue)
      (else
        (set `self.LandingPlace` _item_3)
        (return _returnvalue_2)))
    (elif (<= _returnvalue_4 0.66)
      (`SceneComponent.SetVisibility` (`self.powerbar`) false false)
      (set `self.LandingPlace` _item_2)
      (return (`self.K2_GetActorLocation` _item_2))
      (else
        (`SceneComponent.SetVisibility` (`self.powerbar`) false false)
        (if _returnvalue_3
          (set `self.LandingPlace` _item_3)
          (return _returnvalue_2)
          (else
            (set `self.LandingPlace` _item)
            (return _returnvalue)))))))

(fn `findGoldenGlobe`
  (bind _landingplace (`self.LandingPlace`))
  (bind _outactors (`GameplayStatics.GetAllActorsOfClass` "/Game/Blueprints/RoundControllerNext.RoundControllerNext_C"))
  (bind _item (`KismetArrayLibrary.Array_Get` _outactors))
  (if (or (== (`/Game/Blueprints/RoundControllerNext.item1` _item) _landingplace) (== (`/Game/Blueprints/RoundControllerNext.item2` _item) _landingplace))
    (`|SpawnActorFromClass` "/Game/Blueprints/goldenGlobe/goldenBall.goldenBall_C" (`self.GetTransform` self) "AlwaysSpawn" "OverrideRootScale")))

(fn `shockwaveActivate`
  (bind _shockwave (`self.shockwave`))
  (`ParticleSystemComponent.SetFloatParameter` _shockwave "life" 20.0)
  (`ActorComponent.Activate` _shockwave true))

(fn `UserConstructionScript`)