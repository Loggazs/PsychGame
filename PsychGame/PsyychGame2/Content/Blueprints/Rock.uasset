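; Rock is a scattered grid tile actor in a round-based colour-salience experiment that can be highlighted, blink, vanish or break when the player lands.
; RoundControllerNext's current data row supplies the non-salient CIELAB colour, converted to RGB.
; Playerlanding grows a neighbour set by Force using fixed array-index offsets, trims it by distance, dooms those rocks, then notifies the controller.
; Doomed rocks swap to a destructible cake mesh and spawn chocolate or fruit, depending on CheckLanding.
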(event `make Salient`
  (params (color :type "Vector Structure"))
  (bind _destructible (`self.Destructible`))
  (bind _staticmeshcomponent (`self.StaticMeshComponent`))
  ;[1 1 1] salientColor
  (`PrimitiveComponent.SetMaterial` _staticmeshcomponent 0 "/Game/CustomMaterial/Color.Color")
  (`MeshComponent.SetVectorParameterValueOnMaterials` _staticmeshcomponent "Base" color)
  (`PrimitiveComponent.SetMaterial` _destructible 0 "/Game/CustomMaterial/Color.Color")
  (`MeshComponent.SetVectorParameterValueOnMaterials` _destructible "Base" color)
  (set `self.isSalient` true))

(event `self.ReceiveBeginPlay`
  (if (`self.PlayerRock`)
    (`self.K2_SetActorLocation` (0.0 0.0 0.0))
    (`self.SetActorHiddenInGame` true)))

(event `makeNotSalient`
  (bind _destructible (`self.Destructible`))
  (bind _staticmeshcomponent (`self.StaticMeshComponent`))
  ;[1 1 1] nonSalientColor
  (bind _outactors (`GameplayStatics.GetAllActorsOfClass` "/Game/Blueprints/RoundControllerNext.RoundControllerNext_C"))
  (bind _returnvalue (`|GetDataTableRow` "/Game/Data/ExperimentData.ExperimentData" (`/Game/Blueprints/RoundControllerNext.CurrentRow` (`KismetArrayLibrary.Array_Get` _outactors)))
    (:`then`
      (bind _rgb (`/Game/Blueprints/changeColor.CIELABtoRGB` (`.Color1_30_C866E2DD40B1CB230D71999A96C1B356` (break `/Game/Data/ExperimentParameters` _returnvalue))))
      (`PrimitiveComponent.SetMaterial` _staticmeshcomponent 0 "/Game/CustomMaterial/Color.Color")
      (`MeshComponent.SetVectorParameterValueOnMaterials` _staticmeshcomponent "Base" _rgb)
      (`PrimitiveComponent.SetMaterial` _destructible 0 "/Game/CustomMaterial/Color.Color")
      (`MeshComponent.SetVectorParameterValueOnMaterials` _destructible "Base" _rgb))))

(event `rumble`
  ;[1 1 1] attention Effect
  (`SceneComponent.SetVisibility` (`self.StaticMeshComponent`) false false)
  (`KismetSystemLibrary.Delay` 0.2)
  (`SceneComponent.SetVisibility` (`self.StaticMeshComponent`) true false))

(event `Playerlanding`
  (params (force :type Integer))
  ;[1 1 1] player lands on target
  (bind _outactors (`GameplayStatics.GetAllActorsOfClass` "/Game/Blueprints/RoundControllerNext.RoundControllerNext_C"))
  (bind _item (`KismetArrayLibrary.Array_Get` _outactors))
  (set `/Game/Blueprints/RoundControllerNext.PlayerPosition` self _item)
  (`self.createArrayForDestruction` force)
  (`self.cutNeighbours` (`KismetMathLibrary.Conv_IntToDouble` force))
  (for _array_element (`self.effectedRocks`)
    (`self.selectedForDoom` _array_element))
  (`KismetSystemLibrary.Delay` 1.0)
  (`/Game/Blueprints/RoundControllerNext.Player Landed` _item))

(event `disapear`
  (bind _scattervalue (`self.scatterValue`))
  (bind _returnvalue (* _scattervalue -1.0))
  ;[1 1 1] disapearAction
  (`GameplayStatics.SpawnEmitterAtLocation` "/Game/misc/poof.poof" (+ (`self.K2_GetActorLocation` self) (0.0 0.0 50.0)) (struct) false)
  (`KismetSystemLibrary.Delay` 1.0)
  (`SceneComponent.SetVisibility` (`self.StaticMeshComponent`) false false)
  (`self.makeNotSalient`)
  (`self.K2_SetActorLocation` (+ (`self.Position`) (`KismetMathLibrary.MakeVector` (`KismetMathLibrary.RandomFloatInRange` _returnvalue _scattervalue) (`KismetMathLibrary.RandomFloatInRange` _returnvalue _scattervalue)))))

(event `selectedForDoom`
  (bind (_returnvalue_location _returnvalue_rotation) (`KismetMathLibrary.BreakTransform` (`self.GetTransform` self)))
  (bind _returnvalue (+ _returnvalue_location (60.0 0.0 120.0)))
  ;[1 1 1] action when rock is supposed to go kaputt
  (`SceneComponent.SetVisibility` (`self.StaticMeshComponent`) false false)
  (`DestructibleComponent.SetDestructibleMesh` (`self.Destructible`) "/Game/cupcake/singleCake_DM.singleCake_DM")
  (bind _asplayer_next (cast `/Game/Blueprints/PlayerNext` (`GameplayStatics.GetPlayerPawn` 0)))
  (bind _rightone (`/Game/Blueprints/PlayerNext.checkLanding` _asplayer_next))
  (if _rightone
    (`|SpawnActorFromClass` "/Game/Blueprints/choclatechip.choclatechip_C" (`KismetMathLibrary.MakeTransform` _returnvalue _returnvalue_rotation) "Undefined" "OverrideRootScale")
    (else
      (`|SpawnActorFromClass` "/Game/Blueprints/fruitPiece.fruitPiece_C" (`KismetMathLibrary.MakeTransform` _returnvalue _returnvalue_rotation) "Undefined" "OverrideRootScale"))))

(fn `createArrayForDestruction`
  (params (force :type Integer))
  (bind _counthits (`self.countHits`))
  (if (== _counthits force)
    (if (== _counthits 0)
      (`/Engine/EditorBlueprintResources/StandardMacros.DoOnce` false
        (:`Completed`
          (`KismetArrayLibrary.Array_Add` (`self.effectedRocks`) self)
          (`/Engine/EditorBlueprintResources/StandardMacros.IncrementInt` (`self.countHits`))))
      (else
        (for _array_element (`self.effectedRocks`)
          (bind _effectedrocks (`self.getNeighboursSimple` _array_element))
          (for _array_element_2 _effectedrocks
            (`KismetArrayLibrary.Array_AddUnique` (`self.bufferArray`) _array_element_2)))
        (for _array_element_3 (`self.bufferArray`)
          (`KismetArrayLibrary.Array_AddUnique` (`self.effectedRocks`) _array_element_3))
        (`/Engine/EditorBlueprintResources/StandardMacros.IncrementInt` (`self.countHits`))))
    (else
      (while (<= (`self.countHits`) force)
        (switch `int` (`self.countHits`)
          (:`0`
            (`KismetArrayLibrary.Array_Add` (`self.effectedRocks`) self)
            (`/Engine/EditorBlueprintResources/StandardMacros.IncrementInt` (`self.countHits`)))
          (:`1`
            (`/Engine/EditorBlueprintResources/StandardMacros.DoOnce` false :!label _label
              (:`Completed`
                (for _array_element_4 (`self.effectedRocks`)
                  (bind _effectedrocks_2 (`self.getNeighboursSimple` _array_element_4))
                  (for _array_element_5 _effectedrocks_2
                    (`KismetArrayLibrary.Array_AddUnique` (`self.bufferArray`) _array_element_5)))
                (for _array_element_6 (`self.bufferArray`)
                  (`KismetArrayLibrary.Array_AddUnique` (`self.effectedRocks`) _array_element_6))
                (`/Engine/EditorBlueprintResources/StandardMacros.IncrementInt` (`self.countHits`)))))
          (:`2`
            (`/Engine/EditorBlueprintResources/StandardMacros.DoOnce` false
              (:`Completed`
                (`|ExecutionSequence`
                  (:`then_0`
                    (goto _label :!via `Reset`))
                  (:`then_1`
                    (goto _label))))))
          (:`3`
            (`/Engine/EditorBlueprintResources/StandardMacros.DoOnce` false
              (:`Completed`
                (`|ExecutionSequence`
                  (:`then_0`
                    (goto _label :!via `Reset`))
                  (:`then_1`
                    (goto _label))))))
          (:`4`
            (`/Engine/EditorBlueprintResources/StandardMacros.DoOnce` false
              (:`Completed`
                (`|ExecutionSequence`
                  (:`then_0`
                    (goto _label :!via `Reset`))
                  (:`then_1`
                    (goto _label))))))
          (:`5`
            (`/Engine/EditorBlueprintResources/StandardMacros.DoOnce` false
              (:`Completed`
                (`|ExecutionSequence`
                  (:`then_0`
                    (goto _label :!via `Reset`))
                  (:`then_1`
                    (goto _label))))))
          (:`6`
            (`/Engine/EditorBlueprintResources/StandardMacros.DoOnce` false
              (:`Completed`
                (`|ExecutionSequence`
                  (:`then_0`
                    (goto _label :!via `Reset`))
                  (:`then_1`
                    (goto _label))))))
          (:`7`
            (`/Engine/EditorBlueprintResources/StandardMacros.DoOnce` false
              (:`Completed`
                (`|ExecutionSequence`
                  (:`then_0`
                    (goto _label :!via `Reset`))
                  (:`then_1`
                    (goto _label)))))))))))

(fn `cutNeighbours`
  (params (force :type "Float (double-precision)"))
  (bind _effectedrocks (`self.effectedRocks`))
  (bind _effectedrocks_2 (`self.effectedRocks`))
  (`KismetSystemLibrary.PrintString` (`KismetStringLibrary.Conv_IntToString` (`KismetArrayLibrary.Array_Length` _effectedrocks)) true true (struct :`G` 0.66 :`B` 1.0 :`A` 1.0) 2000000.0)
  (for _array_element _effectedrocks
    (if (>= (`self.GetHorizontalDistanceTo` _array_element) (* force (`self.distanceBetweenNeighbours`)))
      (`KismetArrayLibrary.Array_AddUnique` (`self.bufferArray2`) _array_element)))
  (for _array_element_2 (`self.bufferArray2`)
    (`KismetArrayLibrary.Array_RemoveItem` _effectedrocks_2 _array_element_2))
  (`KismetArrayLibrary.Array_AddUnique` _effectedrocks_2 self))

(fn `getNeighbours`
  (params (traget :type "/Game/Blueprints/Rock Object Reference"))
  (returns (effectedCakes :type "Array of /Game/Blueprints/Rock Object Reference"))
  (bind _outactors (`GameplayStatics.GetAllActorsOfClass` "Rock_C"))
  (bind _returnvalue (`KismetArrayLibrary.Array_Find` _outactors traget))
  (bind _returnvalue_2 (- (`KismetArrayLibrary.Array_Length` _outactors) 1))
  (bind _item (`KismetArrayLibrary.Array_Get` _outactors (`KismetMathLibrary.Clamp` (+ _returnvalue -1) 0 _returnvalue_2)))
  (bind _returnvalue_3 (`KismetMathLibrary.Abs` (`self.GetHorizontalDistanceTo` traget _item)))
  (if (> _returnvalue_3 (`self.distanceBetweenNeighbours`))
    (bind _item_2 (`KismetArrayLibrary.Array_Get` _outactors (`KismetMathLibrary.Clamp` (+ _returnvalue -17) 0 _returnvalue_2)))
    (bind _item_3 (`KismetArrayLibrary.Array_Get` _outactors (`KismetMathLibrary.Clamp` (+ _returnvalue 1) 0 _returnvalue_2)))
    (bind _item_4 (`KismetArrayLibrary.Array_Get` _outactors (`KismetMathLibrary.Clamp` (+ _returnvalue 17) 0 _returnvalue_2)))
    (bind _array (`|MakeArray` _item _item_2 _item_3 _item_4))
    (`KismetArrayLibrary.Array_RemoveItem` _array _item)
    (bind _returnvalue_4 (`KismetStringLibrary.Conv_DoubleToString` _returnvalue_3))
    (`KismetSystemLibrary.PrintString` _returnvalue_4 true true (struct :`R` 1.0 :`A` 1.0))
    (else
      (`KismetSystemLibrary.PrintString` _returnvalue_4 true true (struct :`G` 0.66 :`B` 1.0 :`A` 1.0) 200.0)))
  (bind _returnvalue_5 (`KismetMathLibrary.Abs` (`self.GetHorizontalDistanceTo` traget _item_2)))
  (if (> _returnvalue_5 (`self.distanceBetweenNeighbours`))
    (`KismetArrayLibrary.Array_RemoveItem` _array _item_2)
    (bind _returnvalue_6 (`KismetStringLibrary.Conv_DoubleToString` _returnvalue_5))
    (`KismetSystemLibrary.PrintString` _returnvalue_6 true true (struct :`R` 1.0 :`A` 1.0))
    (else
      (`KismetSystemLibrary.PrintString` _returnvalue_6)))
  (bind _returnvalue_7 (`KismetMathLibrary.Abs` (`self.GetHorizontalDistanceTo` traget _item_3)))
  (if (> _returnvalue_7 (`self.distanceBetweenNeighbours`))
    (`KismetArrayLibrary.Array_RemoveItem` _array _item_4)
    (bind _returnvalue_8 (`KismetStringLibrary.Conv_DoubleToString` _returnvalue_7))
    (`KismetSystemLibrary.PrintString` _returnvalue_8 true true (struct :`R` 1.0 :`A` 1.0))
    (else
      (`KismetSystemLibrary.PrintString` _returnvalue_8)))
  (bind _returnvalue_9 (`KismetMathLibrary.Abs` (`self.GetHorizontalDistanceTo` traget _item_4)))
  (if (> _returnvalue_9 (`self.distanceBetweenNeighbours`))
    (`KismetArrayLibrary.Array_RemoveItem` _array _item_4)
    (bind _returnvalue_10 (`KismetStringLibrary.Conv_DoubleToString` _returnvalue_9))
    (`KismetSystemLibrary.PrintString` _returnvalue_10 true true (struct :`R` 1.0 :`A` 1.0))
    (else
      (`KismetSystemLibrary.PrintString` _returnvalue_10)))
  (return _array))

(fn `getNeighboursSimple`
  (params (target :type "/Game/Blueprints/Rock Object Reference"))
  (returns (effectedRocks :type "Array of /Game/Blueprints/Rock Object Reference"))
  (bind _outactors (`GameplayStatics.GetAllActorsOfClass` "Rock_C"))
  (bind _returnvalue (`KismetArrayLibrary.Array_Find` _outactors target))
  (bind _returnvalue_2 (- (`KismetArrayLibrary.Array_Length` _outactors) 1))
  (return (`|MakeArray` (`KismetArrayLibrary.Array_Get` _outactors (`KismetMathLibrary.Clamp` (+ _returnvalue -1) 0 _returnvalue_2)) (`KismetArrayLibrary.Array_Get` _outactors (`KismetMathLibrary.Clamp` (+ _returnvalue -17) 0 _returnvalue_2)) (`KismetArrayLibrary.Array_Get` _outactors (`KismetMathLibrary.Clamp` (+ _returnvalue 1) 0 _returnvalue_2)) (`KismetArrayLibrary.Array_Get` _outactors (`KismetMathLibrary.Clamp` (+ _returnvalue 17) 0 _returnvalue_2)))))

(fn `UserConstructionScript`
  (bind _returnvalue (`self.K2_GetActorLocation`))
  (bind _scattervalue (`self.scatterValue`))
  (bind _returnvalue_2 (* _scattervalue -1.0))
  ;[1 1 1] Level Setup
  (if (`self.PlayerRock`)
    (`self.K2_SetActorLocation` (0.0 0.0 0.0))
    (`self.SetActorHiddenInGame` true)
    (else
      (set `self.Position` _returnvalue)
      (`self.K2_SetActorLocation` (+ _returnvalue (`KismetMathLibrary.MakeVector` (`KismetMathLibrary.RandomFloatInRange` _returnvalue_2 _scattervalue) (`KismetMathLibrary.RandomFloatInRange` _returnvalue_2 _scattervalue))))
      (`self.makeNotSalient`))))