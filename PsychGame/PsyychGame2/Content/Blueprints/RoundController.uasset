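; RoundController runs the spawn loop for rounds, placing numbered Collison actors at four fixed points around the origin.
; BeginPlay starts a random MultiGate that picks an unused side, spawns there, and re-enters after brief random delays until the count exceeds Phase.
; Each newPhase call counts toward the spawned total; on reaching it, the counters and gate reset and spawning restarts.
; Phase stays at its initial value within this graph.
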(event `self.ReceiveBeginPlay`
  ;[1 1 1] Gameloop v.01
  (`KismetSystemLibrary.Delay` 1.3)
  (set `self.counter` 0)
  (set `self.phase` 1)
  (set `self.destroyCount` 0)
  (`|MultiGate` true :!label _label
    (:`Out 0`
      (set `self.SpawnPoint` (`KismetMathLibrary.MakeTransform` (0.0 350.0 70.0) (struct) (1.0 1.0 1.0))))
    (:`Out 1`
      (set `self.SpawnPoint` (`KismetMathLibrary.MakeTransform` (0.0 -350.0 70.0))))
    (:`Out 2`
      (set `self.SpawnPoint` (`KismetMathLibrary.MakeTransform` (350.0 0.0 70.0))))
    (:`Out 3`
      (set `self.SpawnPoint` (`KismetMathLibrary.MakeTransform` (-350.0 0.0 70.0)))))
  (bind _returnvalue (`|SpawnActorFromClass` "/Game/Blueprints/Collison.Collison_C" (`self.SpawnPoint`) "Undefined" "OverrideRootScale"))
  (bind _output_get (set `/Game/Blueprints/Collison.spawnNumber` (`self.Spawns`) _returnvalue))
  (set `self.Spawns` (+ _output_get 1))
  (bind _output_get_2 (set `self.counter` (+ (`self.counter`) 1)))
  (if (<= _output_get_2 (`self.phase`))
    (`KismetSystemLibrary.Delay` (* (`KismetMathLibrary.RandomFloat`) 0.1))
    (goto _label)))

(event `newPhase`
  ;[1 1 1] Gameloop v.01
  (set `self.Spawns` 1)
  (bind _output_get (set `self.destroyCount` (+ (`self.destroyCount`) 1)))
  (if (>= _output_get (`self.counter`))
    (`KismetSystemLibrary.Delay` 1.0)
    (set `self.counter` 0)
    (set `self.destroyCount` 0)
    (`|ExecutionSequence`
      (:`then_0`
        (goto _label :!via `Reset`))
      (:`then_1`
        (goto _label)))))

(fn `UserConstructionScript`)