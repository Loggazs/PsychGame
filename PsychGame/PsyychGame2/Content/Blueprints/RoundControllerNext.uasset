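; Round controller for an experiment-style game on a rock grid, where two rocks in different random directions rumble each round.
; BeginPlay spawns the grid around the player's rock and fills four directional candidate arrays.
; Each round reads an ExperimentData row for the salient colour and SOA timing, opens matching player directions, then randomly picks an unused row.
; Landing hides rocks and jumps the player back; Space release restores rocks, checks globe power-ups and starts another round.
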(event `RoundStart`
  (bind _loop1 (`self.loop1`))
  (bind _firstset (`self.firstSet`))
  (bind _firsteffect (`self.firstEffect`))
  (bind _donerows (`self.doneRows`))
  (bind _item (`KismetArrayLibrary.Array_Get` (`self.North`) (`KismetMathLibrary.RandomIntegerInRange` 0 2)))
  (bind _item_2 (`KismetArrayLibrary.Array_Get` (`self.East`) (`KismetMathLibrary.RandomIntegerInRange` 0 2)))
  (bind _item_3 (`KismetArrayLibrary.Array_Get` (`self.South`) (`KismetMathLibrary.RandomIntegerInRange` 0 2)))
  (bind _item_4 (`KismetArrayLibrary.Array_Get` (`self.West`) (`KismetMathLibrary.RandomIntegerInRange` 0 2)))
  (`|ExecutionSequence`
    (:`then_0`
      (goto _label :!via `Reset`))
    (:`then_1`
      ;[1 1 1] Choose the two Elements which will display effect per round
      (`|MultiGate` true :!label _label
        (:`Out 0`
          (if _firstset
            (set `self.item2` _item)
            (else
              (set `self.item1` _item))))
        (:`Out 1`
          (if _firstset
            (set `self.item2` _item_2)
            (else
              (set `self.item1` _item_2))))
        (:`Out 2`
          (if _firstset
            (set `self.item2` _item_3)
            (else
              (set `self.item1` _item_3))))
        (:`Out 3`
          (if _firstset
            (set `self.item2` _item_4)
            (else
              (set `self.item1` _item_4)))))
      (if (< _loop1 1.0)
        (set `self.firstSet` true)
        (`/Engine/EditorBlueprintResources/StandardMacros.IncrementFloat` _loop1
          (:`  `
            (goto _label)))
        (else
          (set `self.firstSet` false)
          (set `self.loop1` 0.0)
          (`KismetSystemLibrary.Delay` 0.001)
          (bind _returnvalue (`|GetDataTableRow` "/Game/Data/ExperimentData.ExperimentData" (`self.CurrentRow`))
            (:`then`
              (bind _rgb (`/Game/Blueprints/changeColor.CIELABtoRGB` (`.Color2_31_87878DC947937F3189B87EA4C9B2E2F9` (break `/Game/Data/ExperimentParameters` _returnvalue))))
              (bind _asrock (cast `/Game/Blueprints/Rock` (`self.item2`)))
              (`/Game/Blueprints/Rock.make Salient` _asrock _rgb)
              (`self.openControlls`)
              (`KismetSystemLibrary.Delay` 2.0)
              (bind _returnvalue_2 (+ (* (break `/Game/Data/ExperimentParameters` _returnvalue) 0.001) 0.15))
              (if (> _returnvalue_2 0.15)
                (set `self.2ndElement` (`self.item1`))
                (else
                  (set `self.2ndElement` (`self.item2`))))
              (`|ExecutionSequence`
                (:`then_0`
                  (`KismetSystemLibrary.Delay` 0.15)
                  (bind _asrock_2 (cast `/Game/Blueprints/Rock` (`self.item2`)))
                  (`/Game/Blueprints/Rock.rumble` _asrock_2)
                  (if _firsteffect
                    (set `self.firstEffect` false :!label _label_2)
                    (while (`KismetArrayLibrary.Array_Contains` _donerows (`self.CurrentRow`))
                      (`self.setCurrRow`))
                    (`KismetArrayLibrary.Array_Add` _donerows (`self.CurrentRow`))
                    (else
                      (set `self.firstEffect` true :!label _label_3))))
                (:`then_1`
                  (`KismetSystemLibrary.Delay` _returnvalue_2)
                  (bind _asrock_3 (cast `/Game/Blueprints/Rock` (`self.item1`)))
                  (`/Game/Blueprints/Rock.rumble` _asrock_3)
                  (if _firsteffect
                    (goto _label_2)
                    (else
                      (goto _label_3))))))))))))

(event `self.ReceiveBeginPlay`
  (bind _returnvalue (`KismetMathLibrary.MakeTransform` (`KismetMathLibrary.MakeVector` (`self.PositionX`) (`self.PositionY`)) (struct) (1.0 1.0 1.0)))
  (bind _newparam (`self.setCurrRow`))
  ;[1 1 1] create field
  (`KismetArrayLibrary.Array_Add` (`self.doneRows`) _newparam)
  (while (<= (`self.loop1`) 16.0)
    (while (<= (`self.loop2`) 16.0)
      (if (and (== (`self.loop1`) 8.0) (== (`self.loop2`) 8.0))
        (if (not (`KismetSystemLibrary.IsValid` (`self.PlayerPosition`)))
          (bind _returnvalue_2 (`|SpawnActorFromClass` "/Game/Blueprints/cake.cake_C" _returnvalue "Undefined" "OverrideRootScale"))
          (set `/Game/Blueprints/Rock.PlayerRock` true _returnvalue_2)
          (set `self.PlayerPosition` _returnvalue_2)
          (set `self.PositionY` (+ (`self.PositionY`) (`self.positionMod`)) :!label _label_4)
          (`/Engine/EditorBlueprintResources/StandardMacros.IncrementFloat` (`self.loop2`)))
        (else
          (bind _returnvalue_3 (`|SpawnActorFromClass` "/Game/Blueprints/Rock.Rock_C" _returnvalue "Undefined" "OverrideRootScale"))
          (if (and (== (`self.loop2`) 8.0) (`KismetMathLibrary.InRange_FloatFloat` (`self.loop1`) 2.0 4.0))
            (`KismetArrayLibrary.Array_Add` (`self.North`) _returnvalue_3)
            (goto _label_4)
            (elif (and (`KismetMathLibrary.InRange_FloatFloat` (`self.loop2`) 12.0 14.0) (== (`self.loop1`) 8.0))
              (`KismetArrayLibrary.Array_Add` (`self.East`) _returnvalue_3)
              (goto _label_4)
              (elif (and (== (`self.loop2`) 8.0) (`KismetMathLibrary.InRange_FloatFloat` (`self.loop1`) 12.0 14.0))
                (`KismetArrayLibrary.Array_Add` (`self.South`) _returnvalue_3)
                (goto _label_4)
                (elif (and (`KismetMathLibrary.InRange_FloatFloat` (`self.loop2`) 2.0 4.0) (== (`self.loop1`) 8.0))
                  (`KismetArrayLibrary.Array_Add` (`self.West`) _returnvalue_3)
                  (goto _label_4)
                  (else
                    (goto _label_4)))))))))
    (set `self.PositionX` (+ (`self.PositionX`) (* (`self.positionMod`) -1.0)))
    (set `self.PositionY` -1800.0)
    (set `self.loop2` 0.0)
    (`/Engine/EditorBlueprintResources/StandardMacros.IncrementFloat` (`self.loop1`)))
  (set `self.loop1` 0.0)
  (set `self.loop2` 0.0)
  (set `self.PositionX` 1800.0) ; Ende der Levelerstellung
  (`self.RoundStart`))

(event `Key|SpaceBar` :paused true
  (params (Key :type "Key Structure" :default "AnyKey"))
  (:`Released`
    (`self.closeControlls`)
    (`self.globeCollectionCheck`)
    (bind _outactors (`GameplayStatics.GetAllActorsOfClass` "/Game/Blueprints/Rock.Rock_C"))
    (for _array_element _outactors
      (bind _asrock (cast `/Game/Blueprints/Rock` _array_element))
      (`SceneComponent.SetVisibility` (`StaticMeshActor.StaticMeshComponent` _asrock) true false))
    (for _array_element_2 (`self.doneRows`)
      _)
    (`self.RoundStart`)))

(event `Player Landed`
  (`self.changeRocks`)
  (bind _asplayer_next (cast `/Game/Blueprints/PlayerNext` (`GameplayStatics.GetPlayerCharacter` 0)))
  (`KismetSystemLibrary.Delay` 1.0)
  (`/Game/Blueprints/PlayerNext.jumpBack` _asplayer_next (`self.K2_GetActorLocation` (`self.PlayerPosition`)) (0.0 0.0 0.0)))

(fn `changeRocks`
  (bind _outactors (`GameplayStatics.GetAllActorsOfClass` "/Game/Blueprints/Rock.Rock_C"))
  (for _array_element _outactors
    (`/Game/Blueprints/Rock.disapear` _array_element)))

(fn `closeControlls`
  (bind _asplayer_next (cast `/Game/Blueprints/PlayerNext` (`GameplayStatics.GetPlayerPawn` 0)))
  (`|ExecutionSequence`
    (:`then_0`
      (set `/Game/Blueprints/PlayerNext.North` false _asplayer_next))
    (:`then_1`
      (set `/Game/Blueprints/PlayerNext.East` false _asplayer_next))
    (:`then_2`
      (set `/Game/Blueprints/PlayerNext.South` false _asplayer_next))
    (:`then_3`
      (set `/Game/Blueprints/PlayerNext.West` false _asplayer_next))))

(fn `globeCollectionCheck`
  (if (>= (`self.NumberOfCollectedGlobes`) (`self.GlobePowerUPThreshold`))
    (set `self.GlobePowerUPThreshold` (+ (`self.GlobePowerUPThreshold`) (/ (`self.GlobePowerUPThreshold`) 2)))
    (bind _asplayer_next (cast `/Game/Blueprints/PlayerNext` (`GameplayStatics.GetPlayerPawn` 0)))
    (`/Engine/EditorBlueprintResources/StandardMacros.IncrementInt` (`/Game/Blueprints/PlayerNext.globeStage` _asplayer_next)
      (:`  `
        (bind _hudrreference (`/Game/Blueprints/PlayerNext.HudRreference` _asplayer_next))
        (set `/Game/Blueprints/UI/Hud.GlobeCounter` 0 _hudrreference)
        (`/Game/Blueprints/UI/Hud.removeAllGlobes` _hudrreference)))))

(fn `openControlls`
  (bind _returnvalue (`GameplayStatics.GetPlayerPawn` 0))
  (bind _north (`self.North`))
  (bind _east (`self.East`))
  (bind _south (`self.South`))
  (bind _west (`self.West`))
  (`|ExecutionSequence`
    (:`then_0`
      (if (`KismetArrayLibrary.Array_Contains` _north (`self.item1`))
        (bind _asplayer_next (cast `/Game/Blueprints/PlayerNext` _returnvalue :!label _label))
        (set `/Game/Blueprints/PlayerNext.North` true _asplayer_next)
        (elif (`KismetArrayLibrary.Array_Contains` _north (`self.item2`))
          (goto _label))))
    (:`then_1`
      (if (`KismetArrayLibrary.Array_Contains` _east (`self.item1`))
        (bind _asplayer_next_2 (cast `/Game/Blueprints/PlayerNext` _returnvalue :!label _label_2))
        (set `/Game/Blueprints/PlayerNext.East` true _asplayer_next_2)
        (elif (`KismetArrayLibrary.Array_Contains` _east (`self.item2`))
          (goto _label_2))))
    (:`then_2`
      (if (`KismetArrayLibrary.Array_Contains` _south (`self.item1`))
        (bind _asplayer_next_3 (cast `/Game/Blueprints/PlayerNext` _returnvalue :!label _label_3))
        (set `/Game/Blueprints/PlayerNext.South` true _asplayer_next_3)
        (elif (`KismetArrayLibrary.Array_Contains` _south (`self.item2`))
          (goto _label_3))))
    (:`then_3`
      (if (`KismetArrayLibrary.Array_Contains` _west (`self.item1`))
        (bind _asplayer_next_4 (cast `/Game/Blueprints/PlayerNext` _returnvalue :!label _label_4))
        (set `/Game/Blueprints/PlayerNext.West` true _asplayer_next_4)
        (elif (`KismetArrayLibrary.Array_Contains` _west (`self.item2`))
          (goto _label_4))))))

(fn `setCurrRow`
  (returns (NewParam :type Name))
  (bind _outrownames (`DataTableFunctionLibrary.GetDataTableRowNames` "/Game/Data/ExperimentData.ExperimentData"))
  (bind _output_get (set `self.CurrentRow` (`KismetStringLibrary.Conv_StringToName` (`KismetStringLibrary.Conv_IntToString` (`KismetMathLibrary.RandomIntegerInRange` 1 (`KismetArrayLibrary.Array_Length` _outrownames))))))
  (return _output_get))

(fn `UserConstructionScript`)