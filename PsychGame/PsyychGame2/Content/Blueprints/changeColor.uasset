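; changeColor provides color-space conversion functions that turn a CIELAB vector into an RGB vector.
; CIELABtoRGB chains CIELABtoXYZ, a piecewise inverse Lab transform, into XYZtoRGB, which applies a linear matrix and sRGB gamma.
; Both stages compute channels in Sequence branches and use an AllReady counter to return once all three finish.
; White-point and 255 scaling nodes are unconnected, and the Z term divides (fy − b) by 200, unlike standard fy − b/200.
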(fn CIELABtoXYZ
  (params (cielab :type Vector))
  (bind (_x _y _z) (Math|Vector|BreakVector cielab))
  (bind _returnvalue (/ 16.0 116.0))
  (bind _returnvalue_2 (/ _y 5e+02))
  (bind _returnvalue_3 (+ _x 16.0))
  (bind _returnvalue_4 (/ _returnvalue_3 116.0))
  (bind _returnvalue_5 (- _returnvalue_4 _z))
  (bind _returnvalue_6 (Math|Float|Power _returnvalue_4 3.0))
  (bind _returnvalue_7 (+ _returnvalue_2 _returnvalue_4))
  (bind _returnvalue_8 (Math|Float|Power _returnvalue_7 3.0))
  (bind _returnvalue_9 (/ _returnvalue_5 2e+02))
  (bind _returnvalue_10 (Math|Float|Power _returnvalue_9 3.0))
  (Utilities|FlowControl|Sequence
    (:then_0
      (if (> _returnvalue_6 0.00856)
        (LocalVariables|SetY _returnvalue_6)
        (else
          (LocalVariables|SetY (/ (- _returnvalue_4 _returnvalue) 7.787))))
      (LocalVariables|SetY (LocalVariables|GetY))
      (Math|Integer|IncrementInt (LocalVariables|GetallReady)
        (:%20%20
          _)))
    (:then_1
      (if (> _returnvalue_8 0.008856)
        (LocalVariables|SetX _returnvalue_8)
        (else
          (LocalVariables|SetX (/ (- _returnvalue_7 _returnvalue) 7.787))))
      (LocalVariables|SetX (LocalVariables|GetX))
      (Math|Integer|IncrementInt (LocalVariables|GetallReady)
        (:%20%20
          _)))
    (:then_2
      (if (> _returnvalue_10 0.008856)
        (LocalVariables|SetZ _returnvalue_10)
        (else
          (LocalVariables|SetZ (/ (- _returnvalue_9 _returnvalue) 7.787))))
      (LocalVariables|SetZ (LocalVariables|GetZ))
      (Math|Integer|IncrementInt (LocalVariables|GetallReady)
        (:%20%20
          _))))
  (if (>= (LocalVariables|GetallReady) 3)
    (LocalVariables|SetallReady 0)
    (return (Math|Vector|MakeVector (LocalVariables|GetX) (LocalVariables|GetY) (LocalVariables|GetZ)))))

(fn XYZtoRGB
  (params (XYZ :type Vector))
  (bind (_x _y _z) (Math|Vector|BreakVector XYZ))
  (bind _allready (LocalVariables|GetallReady))
  (Utilities|FlowControl|Sequence
    (:then_0
      (bind _output_get (LocalVariables|SetR (+ (+ (* _x 3.2406) (* _y -1.5372)) (* _z -0.4986))))
      (if (> _output_get 0.0031308)
        (LocalVariables|SetR (- (* 1.055 (Math|Float|Power (LocalVariables|GetR) (/ 1.0 2.4))) 0.055))
        (else
          (LocalVariables|SetR (* (LocalVariables|GetR) 12.92))))
      (LocalVariables|SetR (LocalVariables|GetR))
      (Math|Integer|IncrementInt _allready
        (:%20%20
          _)))
    (:then_1
      (bind _output_get_2 (LocalVariables|SetG (+ (+ (* _x -0.9689) (* _y 1.8758)) (* _z 0.0415))))
      (if (> _output_get_2 0.0031308)
        (LocalVariables|SetG (- (* 1.055 (Math|Float|Power (LocalVariables|GetG) (/ 1.0 2.4))) 0.055))
        (else
          (LocalVariables|SetG (* 12.92 (LocalVariables|GetG)))))
      (LocalVariables|SetG (LocalVariables|GetG))
      (Math|Integer|IncrementInt _allready
        (:%20%20
          _)))
    (:then_2
      (bind _output_get_3 (LocalVariables|SetB (+ (+ (* _x 0.0557) (* _y -0.204)) (* _z 1.057))))
      (if (> _output_get_3 0.0031308)
        (LocalVariables|SetB (- (* 1.055 (Math|Float|Power (LocalVariables|GetB) (/ 1.0 2.4))) 0.055))
        (else
          (LocalVariables|SetB (* 12.92 (LocalVariables|GetB)))))
      (LocalVariables|SetB (LocalVariables|GetB))
      (Math|Integer|IncrementInt _allready
        (:%20%20
          _))))
  (if (>= _allready 3)
    (return (Math|Vector|MakeVector (LocalVariables|GetR) (LocalVariables|GetG) (LocalVariables|GetB)))))

(fn CIELABtoRGB
  (params (CIELAB :type Vector))
  (bind _xyz (CallFunction|CIELABtoXYZ CIELAB))
  (bind _rgb (CallFunction|XYZtoRGB _xyz))
  (return _rgb))