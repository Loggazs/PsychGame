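; Chocolate chip pickup actor that flies to the player and gets eaten shortly after it spawns.
; After a short delay on BeginPlay, the MoveToPlayer timeline lerps it from its current location toward the player pawn each update, tracking the moving target.
; When the timeline finishes, it waits briefly, calls NomNomNom on the PlayerNext pawn and destroys itself.
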(event `self.ReceiveBeginPlay`
  (bind _returnvalue (`GameplayStatics.GetPlayerPawn` 0))
  (`KismetSystemLibrary.Delay` 0.3)
  (bind (_direction _moveit) (`Timeline|move to player`)
    (:`Update`
      (`self.K2_SetActorLocation` (`KismetMathLibrary.VLerp` (`self.K2_GetActorLocation` self) (`self.K2_GetActorLocation` _returnvalue) _moveit)))
    (:`Finished`
      (`KismetSystemLibrary.Delay` 0.1)
      (bind _asplayer_next (cast `/Game/Blueprints/PlayerNext` _returnvalue))
      (`/Game/Blueprints/PlayerNext.NomNomNom` _asplayer_next)
      (`self.K2_DestroyActor`))))

(fn `UserConstructionScript`)