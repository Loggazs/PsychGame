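; Golden globe actor that plays a collection effect as soon as it spawns and calls CollectGoldenGlobe on the PlayerNext pawn's HUD.
; Two chained timelines move it from 100 units above its start: Riseup shifts it along world X and slightly up, then Vibrate offsets it around that point.
; It then swaps the sphere and particles for an explosion and destroys itself after a short delay.
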(event `self.ReceiveBeginPlay`
  (bind _position (`self.position`))
  (bind _explosion (`self.explosion`))
  (bind _position_2 (`self.position`))
  (bind _asplayer_next (cast `/Game/Blueprints/PlayerNext` (`GameplayStatics.GetPlayerPawn` 0)))
  (`/Game/Blueprints/UI/Hud.collectGoldenGlobe` (`/Game/Blueprints/PlayerNext.HudRreference` _asplayer_next))
  (set `self.position` (+ (`self.K2_GetActorLocation`) (0.0 0.0 100.0)))
  (bind (_direction _newtrack_0) (`Timeline|riseup`)
    (:`Update`
      (bind _returnvalue (`KismetMathLibrary.VLerp` _position (+ _position (300.0 0.0 20.0)) _newtrack_0))
      (`self.K2_SetActorLocation` _returnvalue))
    (:`Finished`
      (set `self.position` _returnvalue)
      (bind (_direction_2 _newtrack_7) (`Timeline|vibrate`)
        (:`Update`
          (`self.K2_SetActorLocation` (`KismetMathLibrary.VLerp` _position_2 (+ _position_2 (20.0 20.0 20.0)) _newtrack_7)))
        (:`Finished`
          (`SceneComponent.SetVisibility` _explosion true false)
          (`ActorComponent.SetActive` _explosion true true)
          (`SceneComponent.SetVisibility` (`self.Sphere`) false false)
          (`SceneComponent.SetVisibility` (`self.ParticleSystem`) false false)
          (`KismetSystemLibrary.Delay` 1.5)
          (`self.K2_DestroyActor`))))))

(fn `UserConstructionScript`)